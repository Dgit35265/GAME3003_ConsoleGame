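; BP_TestGameMode is a test game mode that creates the game screen HUD, tracks score and combo, and spawns enemy bots.
; SpawnNewBot runs a single-result EQS query for a spawn location, then SpawnBot places a shotgun humanoid AI there with a debug sphere.
; ResetCombo uses a retriggerable delay to restore the combo multiplier after inactivity.
; ShowWave briefly shows the wave count widget from the HUD.
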(event Custom|ResetCombo
  ;[1 1 1] Reset Combo
  (Utilities|FlowControl|RetriggerableDelay 5.0)
  (Variables|Default|SetComboMultiplier 1))

(event Custom|SpawnBot
  (params (QueryInstance :type Env%20Query%20Instance%20Blueprint%20Wrapper%20Object%20Reference) (QueryStatus :type EEnvQueryStatus%20Enum :default "Processing"))
  (switch Utilities|FlowControl|Switch|SwitchonEEnvQueryStatus QueryStatus
    (:Success
      (bind _resultlocations (AI|EQS|GetQueryResultsasLocations QueryInstance))
      (for _array_element _resultlocations
        (Rendering|Debug|DrawDebugSphere _array_element 1e+02 12 "(R=1.000000,G=0.635953,B=0.000000,A=1.000000)" 5.0 3.0)
        (Game|SpawnActorfromClass "/Game/BluePrint/BP_Test_HumanoidAI_ShotGun.BP_Test_HumanoidAI_ShotGun_C" (Math|Transform|MakeTransform _array_element) "AdjustIfPossibleButAlwaysSpawn" 0 0)))))

(event EventShowWave
  (bind _wavecountuiwidget (Variables|Default|GetWaveCountUIWidget))
  ;[1 1 1] Show Wave Number
  (Widget|SetVisibility _wavecountuiwidget "Visible")
  (Utilities|FlowControl|Delay 4.0)
  (Widget|SetVisibility _wavecountuiwidget "Hidden"))

(event EventTick
  (params (DeltaSeconds :type Float%20%28single-precision%29)))

(event EventSpawnNewBot
  (bind _returnvalue (AI|EQS|RunEQSQuery "/Game/BluePrint/EQS_FindSpawnLocation.EQS_FindSpawnLocation" self "SingleResult"))
  (EventDispatchers|BindEventtoOnQueryFinishedEvent _returnvalue (delegate Custom|SpawnBot)))

(event EventBeginPlay
  ;[1 1 1] Create UI Widget
  (bind _returnvalue (UserInterface|CreateWidget "/Game/UI/GameScreenUI.GameScreenUI_C" (Game|GetPlayerController 0)))
  (bind _output_get (Variables|Default|SetGameScreenUI _returnvalue))
  (UserInterface|Viewport|AddtoViewport _output_get 0)
  (Variables|Default|SetWaveCountUIWidget (Variables|/Game/UI/GameScreenUI.GameScreenUI_C|GetWaveCountUI _output_get))
  (Variables|Default|SetScore 0))

(fn ConstructionScript)