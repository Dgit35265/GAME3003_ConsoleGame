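; Test humanoid AI Blueprint that runs a behavior tree and awards score for kills.
; On BeginPlay it starts Test_BTree and seeds the blackboard with the player pawn as target and its AIClass.
; AddScore adds KillScore times the game mode's combo multiplier, then, only while that multiplier is below 8, doubles it, calls ResetCombo and counts the kill.
; A ShotPoint blackboard update above the player is left unconnected.
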(event EventBeginPlay
  (bind _self self)
  (bind _returnvalue (AI|GetAIController _self))
  (bind _returnvalue_2 (AI|GetBlackboard _returnvalue))
  (AI|RunBehaviorTree _returnvalue "/Game/AI/Test_BTree.Test_BTree")
  (AI|Components|Blackboard|SetValueasObject _returnvalue_2 (Utilities|Name|MakeLiteralName "TargetActor") (Game|Player|GetPlayerPawn 0))
  (AI|Components|Blackboard|SetValueasEnum _returnvalue_2 (Utilities|Name|MakeLiteralName "AIClass") (Variables|Default|GetAIClass)))

(event Collision|EventActorBeginOverlap
  (params (OtherActor :type Actor%20Object%20Reference)))

(event EventTick
  (params (DeltaSeconds :type Float%20%28single-precision%29)))

(event EventAddScore
  ;[1 1 1] Scoring System
  (bind _asbp_test_game_mode (Utilities|Casting|CastToBP_TestGameMode (Game|GetGameMode)))
  (Variables|/Game/BluePrint/BP_TestGameMode.BP_TestGameMode_C|SetScore _asbp_test_game_mode (+ (Variables|/Game/BluePrint/BP_TestGameMode.BP_TestGameMode_C|GetScore _asbp_test_game_mode) (* (Variables|Default|GetKillScore) (Variables|/Game/BluePrint/BP_TestGameMode.BP_TestGameMode_C|GetComboMultiplier _asbp_test_game_mode))))
  (if (< (Variables|/Game/BluePrint/BP_TestGameMode.BP_TestGameMode_C|GetComboMultiplier _asbp_test_game_mode) 8)
    (Variables|/Game/BluePrint/BP_TestGameMode.BP_TestGameMode_C|SetComboMultiplier _asbp_test_game_mode (* (Variables|/Game/BluePrint/BP_TestGameMode.BP_TestGameMode_C|GetComboMultiplier _asbp_test_game_mode) 2))
    (Default|ResetCombo _asbp_test_game_mode)
    (Variables|/Game/BluePrint/BP_TestGameMode.BP_TestGameMode_C|SetTotalKills _asbp_test_game_mode (+ (Variables|/Game/BluePrint/BP_TestGameMode.BP_TestGameMode_C|GetTotalKills _asbp_test_game_mode) 1))))

(fn ConstructionScript)