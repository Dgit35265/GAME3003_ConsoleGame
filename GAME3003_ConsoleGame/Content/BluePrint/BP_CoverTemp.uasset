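; BP_CoverTemp is a cover object that tells third-person characters which cover volume they are standing in.
; Its Front and Back volumes route begin and end overlaps into shared TakeCover and LeaveCover events.
; TakeCover stores the entered volume in the TPScharacter's OverlappingCoverVolume.
; LeaveCover clears it only if it still points to the exited volume, so moving between overlapping sides keeps the newer one.
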(event OnComponentBeginOverlap(Back)
  (params (OverlappedComponent :type Primitive%20Component%20Object%20Reference) (OtherActor :type Actor%20Object%20Reference) (OtherComp :type Primitive%20Component%20Object%20Reference) (OtherBodyIndex :type Integer) (bFromSweep :type Boolean) (SweepResult :type Hit%20Result%20Structure%20%28by%20ref%29))
  (CallFunction|TakeCover OtherActor (Variables|Default|GetBack)))

(event OnComponentBeginOverlap(Front)
  (params (OverlappedComponent :type Primitive%20Component%20Object%20Reference) (OtherActor :type Actor%20Object%20Reference) (OtherComp :type Primitive%20Component%20Object%20Reference) (OtherBodyIndex :type Integer) (bFromSweep :type Boolean) (SweepResult :type Hit%20Result%20Structure%20%28by%20ref%29))
  (CallFunction|TakeCover OtherActor (Variables|Default|GetFront)))

(event OnComponentEndOverlap(Back)
  (params (OverlappedComponent :type Primitive%20Component%20Object%20Reference) (OtherActor :type Actor%20Object%20Reference) (OtherComp :type Primitive%20Component%20Object%20Reference) (OtherBodyIndex :type Integer))
  (CallFunction|LeaveCover OtherActor (Variables|Default|GetBack)))

(event OnComponentEndOverlap(Front)
  (params (OverlappedComponent :type Primitive%20Component%20Object%20Reference) (OtherActor :type Actor%20Object%20Reference) (OtherComp :type Primitive%20Component%20Object%20Reference) (OtherBodyIndex :type Integer))
  (CallFunction|LeaveCover OtherActor (Variables|Default|GetFront)))

(event Custom|TakeCover
  (params (OverlappedActor :type Actor%20Object%20Reference) (OverlappedVolume :type Box%20Component%20Object%20Reference))
  (bind _astpscharacter (Utilities|Casting|CastToTPScharacter OverlappedActor))
  (Variables|/Script/GAME3003_Week01.TPScharacter|SetOverlappingCoverVolume _astpscharacter OverlappedVolume))

(event Custom|LeaveCover
  (params (OverlappedActor :type Actor%20Object%20Reference) (OverlappedVolume :type Box%20Component%20Object%20Reference))
  (bind _astpscharacter (Utilities|Casting|CastToTPScharacter OverlappedActor))
  (if (== (Variables|/Script/GAME3003_Week01.TPScharacter|GetOverlappingCoverVolume _astpscharacter) OverlappedVolume)
    (Variables|/Script/GAME3003_Week01.TPScharacter|SetOverlappingCoverVolume _astpscharacter 0)))

(event EventBeginPlay)

(event Collision|EventActorBeginOverlap
  (params (OtherActor :type Actor%20Object%20Reference)))

(event EventTick
  (params (DeltaSeconds :type Float%20%28single-precision%29)))

(fn ConstructionScript)