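; Third-person shooter player pawn Blueprint whose only live logic creates the GameScreenUI HUD on BeginPlay and adds it to the viewport.
; The remaining graph is disconnected and never runs: cover snapping by line trace, edge-clamped sideways movement, aim-dependent mesh rotation and firing.
; It also holds unwired rifle/launcher swapping, which spawns weapons and attaches them to the mesh's WeaponSocket.
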(event EventBeginPlay
  (bind _returnvalue (UserInterface|CreateWidget "/Game/UI/GameScreenUI.GameScreenUI_C" (Game|GetPlayerController 0)))
  (bind _output_get (Variables|Default|SetHUD _returnvalue))
  (UserInterface|Viewport|AddtoViewport _output_get 0))

(event Input|KeyboardEvents|1
  (params (Key :type Key%20Structure)))

(event Input|KeyboardEvents|2
  (params (Key :type Key%20Structure)))

(fn ConstructionScript)